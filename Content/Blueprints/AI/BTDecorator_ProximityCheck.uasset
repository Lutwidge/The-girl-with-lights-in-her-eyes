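; Behavior tree decorator for monster AI that passes when the controlled pawn is within a set distance of its follow target.
; It casts the owner to BP_AIMonsterController and stores that reference.
; The check compares the distance between the pawn and the blackboard actor under the TargetToFollow key against the Proximity threshold.
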(fn PerformConditionCheck
  (params (OwnerActor :type Actor%20Object%20Reference))
  (bind _asbp_aimonster_controller (Utilities|Casting|CastToBP_AIMonsterController OwnerActor))
  (Variables|Default|SetAI_CON_REF _asbp_aimonster_controller)
  (return (<= (Math|Vector|VectorLength (- (Transformation|GetActorLocation (AI|BehaviorTree|GetBlackboardValueasActor (Variables|Default|GetTargetToFollow))) (Transformation|GetActorLocation (Pawn|GetControlledPawn (Variables|Default|GetAI_CON_REF))))) (Variables|Default|GetProximity))))